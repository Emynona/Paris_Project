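; BP_DecalBasic is a configurable decal Blueprint that applies a textured, tinted material and a size to its DecalBase component.
; Its construction script calls the Color and Size events.
; Color assigns BaseMaterial, creates a dynamic instance, then sets its base color texture and tint parameters.
; Size sets world scale from W on X and a shared UV value on Y and Z, repeating the same call twice.
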(event `Color`
  (`DecalComponent.SetDecalMaterial` (`self.DecalBase`) (`self.BaseMaterial`))
  (bind _returnvalue (`DecalComponent.CreateDynamicMaterialInstance` (`self.DecalBase`)))
  (`MaterialInstanceDynamic.SetTextureParameterValue` _returnvalue "BaseColor" (`self.BaseColorTexture`))
  (`MaterialInstanceDynamic.SetVectorParameterValue` _returnvalue "BaseColor_Tint" (`self.Tint`)))

(event `Size`
  (bind _uv (`self.UV`))
  (bind _w (`self.W`))
  (`SceneComponent.SetWorldScale3D` (`self.DecalBase`) (`KismetMathLibrary.MakeVector` _w _uv _uv))
  (`SceneComponent.SetWorldScale3D` (`self.DecalBase`) (`KismetMathLibrary.MakeVector` _w _uv _uv)))

(fn `UserConstructionScript`
  (locals (NewLocalVar_0 :type "MaterialInterface Object Reference"))
  (`self.Color`)
  (`self.Size`))