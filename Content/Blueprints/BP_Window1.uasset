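; BP_Window1 is a Blueprint window prop that randomizes its look at construction.
; The construction script adds a static mesh component, then assigns Window1 a random mesh from the MeshStore array.
; Window2 randomly receives a mesh from either the MeshPlanks or MeshShutter array.
; The picks are unseeded, so the variant can change whenever construction reruns.
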(event `Window`
  (`AddComponent|NODE_AddStaticMeshComponent-0`))

(event `AddStore`
  (bind _window2 (`self.Window2`))
  (`StaticMeshComponent.SetStaticMesh` (`self.Window1`) (`|GetArrayItem` (`self.MeshStore`) (`KismetMathLibrary.RandomIntegerInRange` 0 4)))
  (switch `int` (`KismetMathLibrary.RandomIntegerInRange` 0 1)
    (:`0`
      (`StaticMeshComponent.SetStaticMesh` _window2 (`|GetArrayItem` (`self.MeshPlanks`) (`KismetMathLibrary.RandomIntegerInRange` 0 4))))
    (:`1`
      (`StaticMeshComponent.SetStaticMesh` _window2 (`|GetArrayItem` (`self.MeshShutter`) (`KismetMathLibrary.RandomIntegerInRange` 0 4))))))

(fn `UserConstructionScript`
  (`self.Window`)
  (`self.AddStore`))