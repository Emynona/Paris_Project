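; Door Blueprint that randomizes its own appearance in the Construction Script.
; SetDoor adds one of four static mesh component variants at random.
; AddPlanks then has a one-in-four chance to put a random MeshPlanks mesh on the StaticMesh component at a fixed relative offset.
; Both rolls use unseeded random integers, so the look can change whenever construction reruns.
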(event `SetDoor`
  (switch `int` (`KismetMathLibrary.RandomIntegerInRange` 0 3)
    (:`0`
      (`AddComponent|NODE_AddStaticMeshComponent-0`))
    (:`1`
      (`AddComponent|NODE_AddStaticMeshComponent-1`))
    (:`2`
      (`AddComponent|NODE_AddStaticMeshComponent-3`))
    (:`3`
      (`AddComponent|NODE_AddStaticMeshComponent-4`))))

(event `AddPlanks`
  (bind _staticmesh (`self.StaticMesh`))
  (switch `int` (`KismetMathLibrary.RandomIntegerInRange` 0 3)
    (:`0`
      (`StaticMeshComponent.SetStaticMesh` _staticmesh (`|GetArrayItem` (`self.MeshPlanks`) (`KismetMathLibrary.RandomIntegerInRange` 0 4)))
      (`SceneComponent.K2_SetRelativeTransform` _staticmesh (`KismetMathLibrary.MakeTransform` (-5.0 0.0 105.0)) false false))))

(fn `UserConstructionScript`
  (`self.SetDoor`)
  (`self.AddPlanks`))