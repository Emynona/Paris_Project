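; BP_HaussmanBuildingWithoutRDC is a building actor that assembles a vertical column of five windows, apparently for a Haussmann-style facade without a ground floor.
; The construction script calls five custom events, each adding a child actor component and attaching it to the root with relative rules.
; Each window has a hardcoded relative position, stacked at roughly even heights, with the top two shifted along X from the lower three.
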(event `AddWindow1`
  (bind _returnvalue (`AddComponent|NODE_AddChildActorComponent-1` :`bManualAttachment` true :`RelativeTransform` (`KismetMathLibrary.MakeTransform` (`KismetMathLibrary.MakeVector` -120.0 0.0 360.0))))
  (`SceneComponent.K2_AttachToComponent` _returnvalue (`self.DefaultSceneRoot`) "None" "KeepRelative" "KeepRelative" "KeepRelative" true))

(event `AddWindow2`
  (bind _returnvalue (`AddComponent|NODE_AddChildActorComponent-2` :`bManualAttachment` true :`RelativeTransform` (`KismetMathLibrary.MakeTransform` (`KismetMathLibrary.MakeVector` -120.0 0.0 660.0))))
  (`SceneComponent.K2_AttachToComponent` _returnvalue (`self.DefaultSceneRoot`) "None" "KeepRelative" "KeepRelative" "KeepRelative" true))

(event `AddWindow3`
  (bind _returnvalue (`AddComponent|NODE_AddChildActorComponent-3` :`bManualAttachment` true :`RelativeTransform` (`KismetMathLibrary.MakeTransform` (`KismetMathLibrary.MakeVector` -120.0 0.0 960.0))))
  (`SceneComponent.K2_AttachToComponent` _returnvalue (`self.DefaultSceneRoot`) "None" "KeepRelative" "KeepRelative" "KeepRelative" true))

(event `AddWindow4`
  (bind _returnvalue (`AddComponent|NODE_AddChildActorComponent-4` :`bManualAttachment` true :`RelativeTransform` (`KismetMathLibrary.MakeTransform` (`KismetMathLibrary.MakeVector` -80.0 0.0 1260.0))))
  (`SceneComponent.K2_AttachToComponent` _returnvalue (`self.DefaultSceneRoot`) "None" "KeepRelative" "KeepRelative" "KeepRelative" true))

(event `AddWindow5`
  (bind _returnvalue (`AddComponent|NODE_AddChildActorComponent-5` :`bManualAttachment` true :`RelativeTransform` (`KismetMathLibrary.MakeTransform` (`KismetMathLibrary.MakeVector` -65.0 0.0 1580.0))))
  (`SceneComponent.K2_AttachToComponent` _returnvalue (`self.DefaultSceneRoot`) "None" "KeepRelative" "KeepRelative" "KeepRelative" true))

(fn `UserConstructionScript`
  (`self.AddWindow1`)
  (`self.AddWindow2`)
  (`self.AddWindow3`)
  (`self.AddWindow4`)
  (`self.AddWindow5`))