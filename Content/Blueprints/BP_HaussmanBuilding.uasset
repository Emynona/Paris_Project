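; Haussmann-style building actor that assembles a door and five stacked windows and varies its point light per instance.
; The construction script attaches each prop as a child actor at a fixed offset and sets the light to either off or a random intensity.
; On BeginPlay, one in six random rolls starts a flicker timeline at a random time, driven by the Intensity variable; other rolls re-randomize the light.
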(event `self.ReceiveBeginPlay`
  (bind _intensity (`self.Intensity`))
  (switch `int` (`KismetMathLibrary.RandomIntegerInRange` 0 5)
    (:`Default`
      (`LightComponent.SetIntensity` (`self.PointLight`) (`|GetArrayItem` (`|MakeArray` (`KismetMathLibrary.RandomFloatInRange` 0.0 4000.0) 0.0) (`KismetMathLibrary.RandomIntegerInRange` 0 1)) :!label _label))
    (:`0`
      (`|ExecutionSequence`
        (:`then_0`
          (bind (_direction _flickering) (`Timeline|Timeline_0` :`NewTime` (`KismetMathLibrary.RandomFloatInRange` 0.0 5.0) :!via `SetNewTime` :!label _label_2)
            (:`Update`
              ;[1 1 1] SetValues
              (`LightComponent.SetIntensity` (`self.PointLight`) (select `bool` (== _flickering 0.0) :`false` _intensity :`true` (`KismetMathLibrary.RandomFloatInRange` 0.0 _intensity))))))
        (:`then_1`
          (goto _label_2))))))

(event `SetLightIntensity`
  (goto _label))

(event `AddDoor`
  ;[1 1 1] Props
  (bind _returnvalue (`AddComponent|NODE_AddChildActorComponent-2` :`bManualAttachment` true :`RelativeTransform` (`KismetMathLibrary.MakeTransform` (`KismetMathLibrary.MakeVector` 78.0))))
  (`SceneComponent.K2_AttachToComponent` _returnvalue (`self.DefaultSceneRoot`) "None" "KeepRelative" "KeepRelative" "KeepRelative" true))

(event `AddWindow1`
  ;[1 1 1] Props
  (bind _returnvalue (`AddComponent|NODE_AddChildActorComponent-3` :`bManualAttachment` true :`RelativeTransform` (`KismetMathLibrary.MakeTransform` (`KismetMathLibrary.MakeVector` -120.0 0.0 360.0))))
  (`SceneComponent.K2_AttachToComponent` _returnvalue (`self.DefaultSceneRoot`) "None" "KeepRelative" "KeepRelative" "KeepRelative" true))

(event `AddWindow2`
  ;[1 1 1] Props
  (bind _returnvalue (`AddComponent|NODE_AddChildActorComponent-5` :`bManualAttachment` true :`RelativeTransform` (`KismetMathLibrary.MakeTransform` (`KismetMathLibrary.MakeVector` -120.0 0.0 660.0))))
  (`SceneComponent.K2_AttachToComponent` _returnvalue (`self.DefaultSceneRoot`) "None" "KeepRelative" "KeepRelative" "KeepRelative" true))

(event `AddWindow3`
  ;[1 1 1] Props
  (bind _returnvalue (`AddComponent|NODE_AddChildActorComponent-7` :`bManualAttachment` true :`RelativeTransform` (`KismetMathLibrary.MakeTransform` (`KismetMathLibrary.MakeVector` -120.0 0.0 960.0))))
  (`SceneComponent.K2_AttachToComponent` _returnvalue (`self.DefaultSceneRoot`) "None" "KeepRelative" "KeepRelative" "KeepRelative" true))

(event `AddWindow4`
  ;[1 1 1] Props
  (bind _returnvalue (`AddComponent|NODE_AddChildActorComponent-8` :`bManualAttachment` true :`RelativeTransform` (`KismetMathLibrary.MakeTransform` (`KismetMathLibrary.MakeVector` -80.0 0.0 1260.0))))
  (`SceneComponent.K2_AttachToComponent` _returnvalue (`self.DefaultSceneRoot`) "None" "KeepRelative" "KeepRelative" "KeepRelative" true))

(event `AddWindow5`
  ;[1 1 1] Props
  (bind _returnvalue (`AddComponent|NODE_AddChildActorComponent-9` :`bManualAttachment` true :`RelativeTransform` (`KismetMathLibrary.MakeTransform` (`KismetMathLibrary.MakeVector` -65.0 0.0 1580.0))))
  (`SceneComponent.K2_AttachToComponent` _returnvalue (`self.DefaultSceneRoot`) "None" "KeepRelative" "KeepRelative" "KeepRelative" true))

(fn `UserConstructionScript`
  (`self.SetLightIntensity`)
  (`self.AddDoor`)
  (`self.AddWindow1`)
  (`self.AddWindow2`)
  (`self.AddWindow3`)
  (`self.AddWindow4`)
  (`self.AddWindow5`))